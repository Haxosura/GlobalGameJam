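; BP_LaughSphere is an actor that awards laugh points to laughing NPCs.
; Half a second after BeginPlay, it runs GiveLaughPoints once, scanning every BP_NPC in the level with GetAllActorsOfClass, with no distance or overlap check.
; Each NPC flagged IsLaughing gains LaughAmount points, has the flag cleared and runs its own UpdateLaughPoints.
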(event `self.ReceiveBeginPlay`
  (`KismetSystemLibrary.Delay` 0.5)
  (`self.GiveLaughPoints`))

(fn `GiveLaughPoints`
  (bind _outactors (`GameplayStatics.GetAllActorsOfClass` "/Game/NPCs/BP_NPC.BP_NPC_C"))
  (for _array_element _outactors
    (if (`/Game/NPCs/BP_NPC.IsLaughing` _array_element)
      (set `MyNPC.LaughPoints` (+ (`MyNPC.LaughPoints` _array_element) (`self.LaughAmount`)) _array_element)
      (set `/Game/NPCs/BP_NPC.IsLaughing` false _array_element)
      (`/Game/NPCs/BP_NPC.UpdateLaughPoints` _array_element))))

(fn `UserConstructionScript`)