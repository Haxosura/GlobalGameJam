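; NPC Blueprint with multi-line dialogue that leads into a joke selection screen.
; An overlap sphere toggles a world widget displaying the NPC's LaughPoints as the third-person character enters or leaves.
; Each Talk event advances through the Dialogue array in a reused WB_Dialogue widget, then swaps it for JokeSelection once the lines run out.
; Leaving SphereDialogue hides the dialogue widget, and the mesh and capsule ignore the camera channel.
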(event `self.ReceiveBeginPlay`
  (`PrimitiveComponent.SetCollisionResponseToChannel` (`self.Mesh`) "ECC_Camera" "ECR_Ignore")
  (`PrimitiveComponent.SetCollisionResponseToChannel` (`self.CapsuleComponent`) "ECC_Camera" "ECR_Ignore")
  (bind _aslaugh_point_widget (cast `/Game/NPCs/LaughPoint_Widget` (`WidgetComponent.GetUserWidgetObject` (`self.Widget`))))
  (bind _output_get (set `self.LaughPointsRef` _aslaugh_point_widget))
  (set `/Game/NPCs/LaughPoint_Widget.Laugh Points` (`KismetTextLibrary.Conv_IntToText` (`self.LaughPoints`)) _output_get))

(event `self.Sphere.OnComponentBeginOverlap`
  (params (OverlappedComponent :type "PrimitiveComponent Object Reference") (OtherActor :type "Actor Object Reference") (OtherComp :type "PrimitiveComponent Object Reference") (OtherBodyIndex :type Integer) (bFromSweep :type Boolean) (SweepResult :type "HitResult Structure (by ref)"))
  (cast `/Game/ThirdPerson/Blueprints/BP_ThirdPersonCharacter` OtherActor)
  (`SceneComponent.SetVisibility` (`self.Widget`) true false)
  (set `/Game/NPCs/LaughPoint_Widget.Laugh Points` (`KismetTextLibrary.Conv_IntToText` (`self.LaughPoints`)) (`self.LaughPointsRef`)))

(event `self.Sphere.OnComponentEndOverlap`
  (params (OverlappedComponent :type "PrimitiveComponent Object Reference") (OtherActor :type "Actor Object Reference") (OtherComp :type "PrimitiveComponent Object Reference") (OtherBodyIndex :type Integer))
  (cast `/Game/ThirdPerson/Blueprints/BP_ThirdPersonCharacter` OtherActor)
  (`SceneComponent.SetVisibility` (`self.Widget`) false false)
  (set `/Game/NPCs/LaughPoint_Widget.Laugh Points` (`KismetTextLibrary.Conv_IntToText` (`self.LaughPoints`)) (`self.LaughPointsRef`)))

(event `/Game/NPCs/Dialogue/BPI_Dialogue.Talk`
  (`/Engine/EditorBlueprintResources/StandardMacros.IncrementInt` (`self.TalkIndex`)
    (:`  `
      (if (< (`self.TalkIndex`) (`KismetArrayLibrary.Array_Length` (`self.Dialogue`)))
        (`self.UIDio`
          (:`then`
            _)
          (:`else`
            (bind _returnvalue (`|CreateWidget` "/Game/BaseProject/UI/NPC_Dialogue/WB_Dialogue.WB_Dialogue_C" (`GameplayStatics.GetPlayerController` 0)))
            (bind _output_get (set `self.UIDio` _returnvalue))
            (`UserWidget.AddToViewport` _output_get 0)))
        (`TextBlock.SetText` (`/Game/BaseProject/UI/NPC_Dialogue/WB_Dialogue.TalkText` (`self.UIDio`)) (`KismetTextLibrary.Conv_StringToText` (`|GetArrayItem` (`self.Dialogue`) (`self.TalkIndex`))))
        (else
          (`Widget.RemoveFromParent` (`self.UIDio`))
          (bind _returnvalue_2 (`|CreateWidget` "/Game/BaseProject/UI/NPC_Dialogue/JokeSelections/jokeSelection.jokeSelection_C"))
          (`UserWidget.AddToViewport` _returnvalue_2 0))))))

(event `self.SphereDialogue.OnComponentEndOverlap`
  (params (OverlappedComponent :type "PrimitiveComponent Object Reference") (OtherActor :type "Actor Object Reference") (OtherComp :type "PrimitiveComponent Object Reference") (OtherBodyIndex :type Integer))
  (`Widget.SetVisibility` (`self.UIDio`) "Hidden"))

(fn `UserConstructionScript`)