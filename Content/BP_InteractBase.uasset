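; BP_InteractBase is an interactable actor base that shows an interaction prompt widget while the player character is within its InteractionSphere.
; It caches the player character on BeginPlay, then creates a new W_Interact widget and sets HitPlayer on each overlap begin.
; On overlap end it removes the widget, clears HitPlayer and resets the cached character's InteractionCounter.
; No interaction action is implemented in this graph.
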(event `self.ReceiveBeginPlay`
  (bind _asbp_third_person_character (cast `/Game/ThirdPerson/Blueprints/BP_ThirdPersonCharacter` (`GameplayStatics.GetPlayerCharacter` 0)))
  (set `self.Player Character` _asbp_third_person_character))

(event `self.InteractionSphere.OnComponentBeginOverlap`
  (params (OverlappedComponent :type "PrimitiveComponent Object Reference") (OtherActor :type "Actor Object Reference") (OtherComp :type "PrimitiveComponent Object Reference") (OtherBodyIndex :type Integer) (bFromSweep :type Boolean) (SweepResult :type "HitResult Structure (by ref)"))
  ;[1 1 1] Player Overlap
  (cast `/Game/ThirdPerson/Blueprints/BP_ThirdPersonCharacter` OtherActor)
  (bind _returnvalue (`|CreateWidget` "/Game/BaseProject/UI/W_Interact.W_Interact_C"))
  (bind _output_get (set `self.Widget` _returnvalue))
  (`UserWidget.AddToViewport` _output_get 0)
  (set `self.HitPlayer` true))

(event `self.InteractionSphere.OnComponentEndOverlap`
  (params (OverlappedComponent :type "PrimitiveComponent Object Reference") (OtherActor :type "Actor Object Reference") (OtherComp :type "PrimitiveComponent Object Reference") (OtherBodyIndex :type Integer))
  ;[1 1 1] Player Overlap
  (cast `/Game/ThirdPerson/Blueprints/BP_ThirdPersonCharacter` OtherActor)
  (`Widget.RemoveFromParent` (`self.Widget`))
  (set `self.HitPlayer` false)
  (set `/Game/ThirdPerson/Blueprints/BP_ThirdPersonCharacter.Interaction Counter` 0 (`self.Player Character`)))

(fn `UserConstructionScript`)